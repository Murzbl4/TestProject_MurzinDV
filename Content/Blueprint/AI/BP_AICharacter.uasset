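; BP_AICharacter is an AI-controlled character Blueprint with a name widget component.
; Its construction script copies the Speed variable into the movement component's max walk speed.
; On BeginPlay, InitWidget casts the NameWidget's widget to WB_NameAI and sets the character as its Owner.
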(event `self.ReceiveBeginPlay`
  (`self.InitWidget`))

(fn `InitWidget`
  (bind _aswb_name_ai (cast `/Game/Blueprint/UI/WB_NameAI` (`WidgetComponent.GetWidget` (`self.NameWidget`))))
  (set `/Game/Blueprint/UI/WB_NameAI.Owner` self _aswb_name_ai))

(fn `UserConstructionScript`
  (set `CharacterMovementComponent.MaxWalkSpeed` (`self.Speed`) (`self.CharacterMovement`)))