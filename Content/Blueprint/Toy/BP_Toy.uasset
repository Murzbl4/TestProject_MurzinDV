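; BP_Toy is a throwable toy actor that awards its points to the AI character that reaches it.
; On a non-player overlap, it refreshes every controller's HUD scoreboard after a short delay.
; If the game state's ThrowToy flag is set and the overlapper is an AI, it adds the score and clears the flag.
; It then sets all AI to waiting, calls ChooseToyServer on every player character and destroys itself.
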(event `UpdateScoreboard`
  (`KismetSystemLibrary.Delay` 0.1)
  (bind _outactors (`GameplayStatics.GetAllActorsOfClass` "/Game/Blueprint/Base/BP_FirstPersonPlayerController.BP_FirstPersonPlayerController_C"))
  (for _array_element _outactors
    (bind _asbp_hud (cast `/Game/Blueprint/Base/BP_HUD` (`PlayerController.GetHUD` _array_element)))
    (`/Game/Blueprint/UI/WB_Scoreboard.refreshList` (`/Game/Blueprint/Base/BP_HUD.ScoreboardRef` _asbp_hud))))

(event `self.Box.OnComponentBeginOverlap`
  (params (OverlappedComponent :type "PrimitiveComponent Object Reference") (OtherActor :type "Actor Object Reference") (OtherComp :type "PrimitiveComponent Object Reference") (OtherBodyIndex :type Integer) (bFromSweep :type Boolean) (SweepResult :type "HitResult Structure (by ref)"))
  (cast `/Game/Blueprint/Character/BP_FirstPersonCharacter` OtherActor
    (:`CastFailed`
      (`self.UpdateScoreboard`)
      (if (`MyGameState.ThrowToy` (`self.As My Game State`))
        (bind _asaicharacter (cast `AICharacter` OtherActor))
        (`PrimitiveComponent.SetCollisionEnabled` (`self.Box`) "NoCollision")
        (set `AICharacter.Score` (+ (`AICharacter.Score` _asaicharacter) (`self.Point`)) _asaicharacter)
        (set `MyGameState.ThrowToy` false (`self.As My Game State`))
        (bind _outactors (`GameplayStatics.GetAllActorsOfClass` "/Game/Blueprint/AI/BP_AICharacter.BP_AICharacter_C"))
        (for _array_element _outactors
          (`AICharacter.SetWaiting` _array_element))
        (bind _outactors_2 (`GameplayStatics.GetAllActorsOfClass` "/Game/Blueprint/Character/BP_FirstPersonCharacter.BP_FirstPersonCharacter_C"))
        (for _array_element_2 _outactors_2
          (`/Game/Blueprint/Character/BP_FirstPersonCharacter.ChooseToy_Server` _array_element_2 0 true))
        (`self.K2_DestroyActor`)))))

(event `self.ReceiveBeginPlay`
  (bind _asmy_game_state (cast `MyGameState` (`GameplayStatics.GetGameState`)))
  (set `self.As My Game State` _asmy_game_state))

(fn `UserConstructionScript`)