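; BP_MyGameState is a game state Blueprint that switches players to the end-game screen.
; Its ShowEndGameUI event loops over every BP_FirstPersonPlayerController, shows the mouse cursor, removes the BP_HUD timer and scoreboard widgets, and disables pawn input.
; For each controller it then creates a WB_EndGame widget with the winner, score and draw flag, and adds it to the viewport.
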(event `self.ShowEndGameUI`
  (params (Winner :type "Actor Object Reference") (Score :type Integer) (bIsDraw :type Boolean))
  (bind _outactors (`GameplayStatics.GetAllActorsOfClass` "/Game/Blueprint/Base/BP_FirstPersonPlayerController.BP_FirstPersonPlayerController_C"))
  (for _array_element _outactors
    (set `PlayerController.bShowMouseCursor` true _array_element)
    (bind _asbp_hud (cast `/Game/Blueprint/Base/BP_HUD` (`PlayerController.GetHUD` _array_element)))
    (`Widget.RemoveFromParent` (`/Game/Blueprint/Base/BP_HUD.TimerRef` _asbp_hud))
    (`Widget.RemoveFromParent` (`/Game/Blueprint/Base/BP_HUD.ScoreboardRef` _asbp_hud))
    (`self.DisableInput` (`Controller.K2_GetPawn` _array_element) _array_element)
    (bind _returnvalue (`|CreateWidget` "/Game/Blueprint/UI/WB_EndGame.WB_EndGame_C" null Score Winner bIsDraw))
    (`/Engine/EditorBlueprintResources/StandardMacros.IsValid` _returnvalue
      (:`Is Valid`
        (`UserWidget.AddToViewport` _returnvalue 0)))))

(fn `UserConstructionScript`)